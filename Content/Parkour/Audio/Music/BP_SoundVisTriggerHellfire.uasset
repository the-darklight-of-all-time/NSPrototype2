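; Music-driven light visualizer actor that plays a sound when VisInt1 fires and modulates every BP_SoundVisHellLights rect light to it.
; Construction script gathers the lights, and the audio playback percent times duration gives the lookup time into pre-analyzed Constant-Q (NRT) data.
; Each band value is scaled, clamped and written to all lights in turn, so the last band wins.
; Lights drop to minimum intensity when audio finishes.
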(event OnAudioFinished(Audio)
  (for _array_element (Variables|Default|GetSoundVisActors)
    (Rendering|Components|Light|SetIntensity (Variables|/Game/Parkour/Audio/Music/BP_SoundVisHellLights.BP_SoundVisHellLights_C|GetRectLight _array_element) (Variables|Default|GetIntensity_Min))))

(event Custom|PlaybackChange
  (params (PlayingSoundWave :type Sound%20Wave%20Object%20Reference) (PlaybackPercent :type Float%20%28single-precision%29))
  (Variables|Default|SetPlayTime (* PlaybackPercent (Variables|Default|GetDuration)))
  (for _array_element (Class|ConstantQNRT|GetNormalizedChannelConstantQatTime (Variables|Default|GetConstant_NRT) (Variables|Default|GetPlayTime))
    (for _array_element_2 (Variables|Default|GetSoundVisActors)
      (Rendering|Components|Light|SetIntensity (Variables|/Game/Parkour/Audio/Music/BP_SoundVisHellLights.BP_SoundVisHellLights_C|GetRectLight _array_element_2) (Math|Float|Clamp(Float) (* _array_element (Variables|Default|GetIntensity_Multiplier)) (Variables|Default|GetIntensity_Min) (Variables|Default|GetIntensity_Max))))))

(event EventBeginPlay
  (bind _sound (Variables|Default|GetSound))
  (Audio|Components|Audio|SetSound (Variables|Default|GetAudio) _sound)
  (Variables|Default|SetDuration (Variables|/Script/Engine.SoundBase|GetDuration _sound)))

(event Collision|EventActorBeginOverlap
  (params (OtherActor :type Actor%20Object%20Reference)))

(event EventTick
  (params (DeltaSeconds :type Float%20%28single-precision%29)))

(event EventVisInt1
  (Variables|Default|SetPlayTime 0.0)
  (EventDispatchers|BindEventtoOnAudioPlaybackPercent (Variables|Default|GetAudio) (delegate Custom|PlaybackChange))
  (Audio|Components|Audio|Play (Variables|Default|GetAudio) 0.0))

(fn ConstructionScript
  (bind _outactors (Actor|GetAllActorsOfClass "/Game/Parkour/Audio/Music/BP_SoundVisHellLights.BP_SoundVisHellLights_C"))
  (Variables|Default|SetSoundVisActors _outactors))