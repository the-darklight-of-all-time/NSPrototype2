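; BP_Telaport is a reset volume that sends the player back to a saved safe location.
; When a BP_ThirdPersonCharacter overlaps its Box, it moves the character to that character's SafeLocation without sweeping and zeroes capsule physics and movement velocity.
; The construction script sets the Box's world transform from Height and Size, setting its Z position and horizontal scale.
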(event OnComponentBeginOverlap(Box)
  (params (OverlappedComponent :type Primitive%20Component%20Object%20Reference) (OtherActor :type Actor%20Object%20Reference) (OtherComp :type Primitive%20Component%20Object%20Reference) (OtherBodyIndex :type Integer) (bFromSweep :type Boolean) (SweepResult :type Hit%20Result%20Structure%20%28by%20ref%29))
  (bind _asbp_third_person_character (Utilities|Casting|CastToBP_ThirdPersonCharacter OtherActor))
  (Transformation|SetActorLocation _asbp_third_person_character (Variables|/Game/ThirdPerson/Blueprints/BP_ThirdPersonCharacter.BP_ThirdPersonCharacter_C|GetSafeLocation _asbp_third_person_character) false false)
  (Class|PrimitiveComponent|SetAllPhysicsLinearVelocity (Variables|/Script/Engine.Character|GetCapsuleComponent _asbp_third_person_character) "0, 0, 0" false)
  (Variables|/Script/Engine.MovementComponent|SetVelocity (Pawn|GetMovementComponent _asbp_third_person_character) "0, 0, 0"))

(fn ConstructionScript
  (bind _size (Variables|Default|GetSize))
  (Transformation|SetWorldTransform (Variables|Default|GetBox) (Math|Transform|MakeTransform (Math|Vector|MakeVector 0.0 0.0 (Variables|Default|GetHeight)) "0, 0, 0" (Math|Vector|MakeVector _size _size 1.0)) false false))