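; BP_OutroTrigger is a trigger actor in the Parkour game that shows the outro screen when the player's pawn overlaps it.
; On overlap it zeroes the character's movement velocity, then creates an outro widget and adds it to the viewport.
; It switches the player controller to UI-only input focused on that widget and shows the mouse cursor.
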(event EventBeginPlay
  ;[0.15 0.15 0.15 0.5] Have the outro widget pop up when this box is triggered, disable player input
)

(event EventTick
  (params (DeltaSeconds :type Float%20%28single-precision%29))
  ;[0.15 0.15 0.15 0.5] Have the outro widget pop up when this box is triggered, disable player input
)

(event Collision|EventActorBeginOverlap
  (params (OtherActor :type Actor%20Object%20Reference))
  (bind _returnvalue (Game|GetPlayerController 0))
  (if (== OtherActor (Game|Player|GetPlayerPawn 0))
    (Variables|/Script/Engine.MovementComponent|SetVelocity (Variables|/Script/Engine.Character|GetCharacterMovement (Game|GetPlayerCharacter 0)) "0, 0, 0")
    (bind _returnvalue_2 (UserInterface|CreateWidget "/Game/Parkour/UI/Widgets/WB_Outro.WB_Outro_C"))
    (UserInterface|Viewport|AddtoViewport _returnvalue_2 0)
    (Input|SetInputModeUIOnly _returnvalue _returnvalue_2 "DoNotLock" false)
    (Variables|/Script/Engine.PlayerController|SetbShowMouseCursor _returnvalue true)))

(fn ConstructionScript)