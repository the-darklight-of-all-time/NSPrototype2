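; BP_FastDialogueTrigger is a trigger volume that shows a short dialogue widget while the player is inside it.
; BeginPlay creates a WB_FastDialogueTrigger widget once and keeps it as InteractWidget.
; When the player character enters the Box, the widget is added to the viewport and receives the trigger's Text, and it is removed when the player leaves.
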(event OnComponentBeginOverlap(Box)
  (params (OverlappedComponent :type Primitive%20Component%20Object%20Reference) (OtherActor :type Actor%20Object%20Reference) (OtherComp :type Primitive%20Component%20Object%20Reference) (OtherBodyIndex :type Integer) (bFromSweep :type Boolean) (SweepResult :type Hit%20Result%20Structure%20%28by%20ref%29))
  (bind _interactwidget (Variables|Default|GetInteractWidget))
  (if (== OtherActor (Game|GetPlayerCharacter 0))
    (UserInterface|Viewport|AddtoViewport _interactwidget 0)
    (Variables|/Game/Parkour/UI/Widgets/WB_FastDialogueTrigger.WB_FastDialogueTrigger_C|SetInputText _interactwidget (Variables|Default|GetText))))

(event OnComponentEndOverlap(Box)
  (params (OverlappedComponent :type Primitive%20Component%20Object%20Reference) (OtherActor :type Actor%20Object%20Reference) (OtherComp :type Primitive%20Component%20Object%20Reference) (OtherBodyIndex :type Integer))
  (if (== (Game|GetPlayerCharacter 0) OtherActor)
    (Widget|RemovefromParent (Variables|Default|GetInteractWidget))))

(event EventBeginPlay
  (bind _returnvalue (UserInterface|CreateWidget "/Game/Parkour/UI/Widgets/WB_FastDialogueTrigger.WB_FastDialogueTrigger_C"))
  (Variables|Default|SetInteractWidget _returnvalue))

(fn ConstructionScript)