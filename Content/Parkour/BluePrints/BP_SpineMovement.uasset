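; Parkour actor that moves a list of actors continuously along a spline, spaced apart by a fixed offset.
; The construction script places each actor at its offset distance along the spline.
; From BeginPlay, a timeline with play rate scaled by TimelineLength advances the actors, setting world location and rotation from the spline and restarting when finished.
; Distances beyond the spline's length wrap with a single subtraction.
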(event Custom|PlayTimeline
  (bind _spline (Variables|Default|GetSpline))
  (bind _spline_2 (Variables|Default|GetSpline))
  (bind _returnvalue (Spline|GetSplineLength _spline))
  (bind _alpha (Timeline|Timeline PlayFromStart)
    (:Update
      (for (_array_element _array_index) (Variables|Default|GetActors)
        (bind _output_get (Variables|Default|SetDistance%20Along%20Spline (+ (Math|Float|Lerp 0.0 (Spline|GetSplineLength (Variables|Default|GetSpline)) _alpha) (* _array_index (Variables|Default|GetOffset%20between%20Actors)))))
        (if (> _output_get _returnvalue)
          (Variables|Default|SetDistance%20Along%20Spline (- (Variables|Default|GetDistance%20Along%20Spline) _returnvalue)))
        (Transformation|SetActorLocationAndRotation _array_element (Spline|GetLocationatDistanceAlongSpline _spline_2 (Variables|Default|GetDistance%20Along%20Spline) "World") (Spline|GetRotationatDistanceAlongSpline _spline_2 (Variables|Default|GetDistance%20Along%20Spline) "World"))))
    (:Finished
      (CallFunction|PlayTimeline))))

(event EventBeginPlay
  (Components|Timeline|SetPlayRate (Variables|Default|GetTimeline) (/ 1.0 (Variables|Default|GettimelineLength)))
  (CallFunction|PlayTimeline))

(fn ConstructionScript
  (bind _spline (Variables|Default|GetSpline))
  (for (_array_element _array_index) (Variables|Default|GetActors)
    (Transformation|SetActorLocationAndRotation _array_element (Spline|GetLocationatDistanceAlongSpline _spline (* (Variables|Default|GetOffset%20between%20Actors) _array_index) "World") (Spline|GetRotationatDistanceAlongSpline _spline (* (Variables|Default|GetOffset%20between%20Actors) _array_index) "World"))))